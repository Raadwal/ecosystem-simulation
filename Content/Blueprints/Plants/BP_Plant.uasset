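; BP_Plant is a spawned plant in a simulation that validates its own placement and reports to the HUD.
; On BeginPlay it takes terrain data from GI_Settings and destroys itself if not above the ocean generator's biome end height.
; It also destroys itself when its collision mesh begins overlapping a TerrainGenerator or another Plant.
; ShowInformationInHUD passes the plant to BP_SimulationHud's widget to display its information.
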(event OnComponentBeginOverlap(_CollisionMeshComponent)
  (params (OverlappedComponent :type Primitive%20Component%20Object%20Reference) (OtherActor :type Actor%20Object%20Reference) (OtherComp :type Primitive%20Component%20Object%20Reference) (OtherBodyIndex :type Integer) (bFromSweep :type Boolean) (SweepResult :type Hit%20Result%20Structure%20%28by%20ref%29))
  ;[1 1 1] Check if spawned plant is colliding with terrain/other plants
  (Utilities|Casting|CastToTerrainGenerator OtherActor
    (:then
      _)
    (:CastFailed
      (Utilities|Casting|CastToPlant OtherActor)))
  (Actor|DestroyActor))

(event EventBeginPlay
  ;[1 1 1] Set Environment Data
  (bind _asgi_settings (Utilities|Casting|CastToGI_Settings (Game|GetGameInstance)))
  (Class|Plant|SetEnvironmentData (Variables|/Game/Blueprints/GI_Settings.GI_Settings_C|GetTerrainData _asgi_settings))
  ;[1 1 1] Check if Plant has been spawned on water
  (bind _returnvalue (Actor|GetActorOfClass "/Game/Blueprints/TerrainGeneration/BP_OceanGenerator.BP_OceanGenerator_C"))
  (if (not (Class|Plant|CheckifAboveGivenTerrainHeight (Variables|/Game/Blueprints/GI_Settings.GI_Settings_C|GetTerrainData _asgi_settings) (Class|TerrainGenerator|GetBiomeEndHeight _returnvalue)))
    (Actor|DestroyActor)))

(fn ConstructionScript)

(fn ShowInformationinHUD
  (bind _returnvalue (Game|GetPlayerController 0))
  (bind _returnvalue_2 (HUD|GetHUD _returnvalue))
  (Utilities|IsValid _returnvalue_2
    (:Is%20Valid
      (bind _asbp_simulation_hud (Utilities|Casting|CastToBP_SimulationHud _returnvalue_2))
      (Default|ShowPlantInformation (Variables|/Game/Blueprints/Widgets/Simulation/BP_SimulationHud.BP_SimulationHud_C|GetSimulationWidget _asbp_simulation_hud) self)
      (return))))